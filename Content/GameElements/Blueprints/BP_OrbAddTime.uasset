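; BP_OrbAddTime is a pickup orb that, judging by its name, grants extra time to the possession ghost.
; When a BP_PossessionGhost overlaps its Sphere, it calls OrbObtained on the ghost, which handles the actual effect.
; The orb then hides its mesh and disables sphere collision, and respawns after a short delay by restoring both.
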(event OnComponentBeginOverlap(Sphere)
  (params (OverlappedComponent :type Primitive%20Component%20Object%20Reference) (OtherActor :type Actor%20Object%20Reference) (OtherComp :type Primitive%20Component%20Object%20Reference) (OtherBodyIndex :type Integer) (bFromSweep :type Boolean) (SweepResult :type Hit%20Result%20Structure%20%28by%20ref%29))
  (bind _asbp_possession_ghost (Utilities|Casting|CastToBP_PossessionGhost OtherActor))
  (Default|OrbObtained _asbp_possession_ghost)
  (Development|SetHiddeninGame (Variables|Default|GetOrb) true false)
  (Collision|SetCollisionEnabled (Variables|Default|GetSphere) "NoCollision")
  (Utilities|FlowControl|Delay 5.0)
  (Development|SetHiddeninGame (Variables|Default|GetOrb) false false)
  (Collision|SetCollisionEnabled (Variables|Default|GetSphere) "QueryAndPhysics"))

(event EventBeginPlay)

(event EventTick
  (params (DeltaSeconds :type Float%20%28single-precision%29)))

(fn ConstructionScript)