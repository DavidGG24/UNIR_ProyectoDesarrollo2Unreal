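; Door that opens when every linked beacon's active state matches the required state set in its Beacons array.
; Each Tick it checks all beacons, stopping at the first mismatch, then plays or reverses the OpenDoor timeline.
; The timeline lerps the WallBot component's relative height to raise or lower it.
; The construction script removes two pillars when WallEndPillars is off.
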(event EventBeginPlay)

(event Collision|EventActorBeginOverlap
  (params (OtherActor :type Actor%20Object%20Reference)))

(event EventTick
  (params (DeltaSeconds :type Float%20%28single-precision%29))
  (bind _wall_bot (Variables|Default|GetWall_bot))
  (bind _relativelocation (Variables|/Script/Engine.SceneComponent|GetRelativeLocation _wall_bot))
  (bind _array_element (Utilities|Array|ForEachLoopwithBreak (Variables|Default|GetBeacons) :!label _label)
    (:LoopBody
      (if (== (Variables|/Game/GameElements/Blueprints/BP_ActivationBeacon.BP_ActivationBeacon_C|GetIsActive (.beacon _array_element)) (.active _array_element))
        (Variables|Default|SetGateIsOpen true)
        (else
          (Variables|Default|SetGateIsOpen false)
          (goto _label Break))))
    (:Completed
      (if (Variables|Default|GetGateIsOpen)
        (bind _newtrack_0 (Timeline|OpenDoor Play)
          (:Update
            (Transformation|SetRelativeLocation _wall_bot (Math|Vector|MakeVector (.x _relativelocation) (.y _relativelocation) (Math|Float|Lerp 0.0 3e+02 _newtrack_0)) false false)))
        (else
          (Timeline|OpenDoor Reverse))))))

(fn ConstructionScript
  (if (not (Variables|Default|GetWallEndPillars))
    (Components|DestroyComponent (Variables|Default|GetPillar_04))
    (Components|DestroyComponent (Variables|Default|GetPillar_03))))