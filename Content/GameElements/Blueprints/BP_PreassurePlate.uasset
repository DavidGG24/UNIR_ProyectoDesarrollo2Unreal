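; Pressure plate Blueprint that toggles a referenced door when something overlaps its capsule.
; Begin and end overlap both call SwitchOnoff on the door, so the door flips again when the overlap ends.
; A timeline lowers the plate mesh slightly on entry and reverses on exit.
; The only gate is a valid player controller 0, so the overlapping actor is never filtered.
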(event OnComponentBeginOverlap(Capsule)
  (params (OverlappedComponent :type Primitive%20Component%20Object%20Reference) (OtherActor :type Actor%20Object%20Reference) (OtherComp :type Primitive%20Component%20Object%20Reference) (OtherBodyIndex :type Integer) (bFromSweep :type Boolean) (SweepResult :type Hit%20Result%20Structure%20%28by%20ref%29))
  (Utilities|IsValid (Game|GetPlayerController 0)
    (:Is%20Valid
      (Default|SwitchOn/off (Variables|Default|GetDoorRef))
      (bind _newtrack_0 (Timeline|TimelinePlate Play)
        (:Update
          (Transformation|SetRelativeLocation (Variables|Default|GetPlate) (Math|Vector|MakeVector 0.0 0.0 (Math|Float|Lerp 0.0 -5.0 _newtrack_0)) false false))))))

(event OnComponentEndOverlap(Capsule)
  (params (OverlappedComponent :type Primitive%20Component%20Object%20Reference) (OtherActor :type Actor%20Object%20Reference) (OtherComp :type Primitive%20Component%20Object%20Reference) (OtherBodyIndex :type Integer))
  (Utilities|IsValid (Game|GetPlayerController 0)
    (:Is%20Valid
      (Default|SwitchOn/off (Variables|Default|GetDoorRef))
      (bind _newtrack_0 (Timeline|TimelinePlate Reverse)
        (:Update
          (Transformation|SetRelativeLocation (Variables|Default|GetPlate) (Math|Vector|MakeVector 0.0 0.0 (Math|Float|Lerp 0.0 -5.0 _newtrack_0)) false false))))))

(event EventBeginPlay)

(event Collision|EventActorBeginOverlap
  (params (OtherActor :type Actor%20Object%20Reference)))

(event EventTick
  (params (DeltaSeconds :type Float%20%28single-precision%29)))

(fn ConstructionScript)